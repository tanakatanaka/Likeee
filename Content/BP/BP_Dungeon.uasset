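; BP_Dungeon is the Blueprint side of a C++ dungeon actor, spawning the grid areas that make up the field.
; On BeginPlay it async-loads the soft BP_GridArea class, caches it, and only then calls MakeField.
; The C++ base calls SpawnAreaBP with horizontal and vertical indices, which spawns a grid area at the scaled world position at a fixed height.
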(event `self.ReceiveBeginPlay`
  (bind _class (`|LoadAssetClass` (`self.sof_bpGridArea`))
    (:`Completed`
      (bind _asbp_grid_area (castclass `/Game/BP/BP_GridArea` _class))
      (set `self.As BP Grid Area` _asbp_grid_area)
      (`self.MakeField`))))

(event `self.SpawnAreaBP`
  (params (horizontal :type Integer) (vertical :type Integer))
  ; call by Base Cpp
  (`|SpawnActorFromClass` (`self.As BP Grid Area`) (`KismetMathLibrary.MakeTransform` (`KismetMathLibrary.MakeVector` (* (`KismetMathLibrary.Conv_IntToDouble` horizontal) 100.0) (* (`KismetMathLibrary.Conv_IntToDouble` vertical) 100.0) 100.0)) "Undefined" "MultiplyWithRoot" null null))

(fn `UserConstructionScript`)